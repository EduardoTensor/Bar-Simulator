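; BP_Spawner is an NPC spawner that keeps at most one tracked BP_NPC at a time.
; On BeginPlay, TrySpawnNPC checks HasNPC and, if false, spawns an NPC at the spawner's transform, passing it an ExitTarget reference.
; It then sets the flag and stores the NPC in CurrentNPC.
; ResetHasNPC clears the flag and immediately retries the spawn, providing a hook for replacement NPCs.
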(event Custom|TrySpawnNPC
  ;[1 1 1] 🇧🇷 Português
  ;
  ; // Sistema de Spawner de NPCs
  ; //
  ; // - Evento BeginPlay: Assim que o jogo começa, chama "Try Spawn NPC".
  ; // - TrySpawnNPC (Evento Personalizado):
  ; //     * Verifica a variável "Has NPC"
  ; //     * Se já existir um NPC (True), não faz nada.
  ; //     * Se não existir (False):
  ; //         - Pega a posição do Spawner (Get Actor Transform).
  ; //         - Cria (Spawn) um novo BP_NPC nessa posição.
  ; //         - Marca "Has NPC" como verdadeiro.
  ; //         - Salva a referência do NPC em "Current NPC".
  ; //
  ; // Resultado: O Spawner só cria NPCs se não houver nenhum ativo.
  ; // Garante controle para evitar spawns duplicados.
  ;
  ; 🇺🇸 English
  ;
  ; // NPC Spawner System
  ; //
  ; // - BeginPlay Event: When the game starts, calls "Try Spawn NPC".
  ; // - TrySpawnNPC (Custom Event):
  ; //     * Checks "Has NPC" variable.
  ; //     * If an NPC already exists (True), does nothing.
  ; //     * If none exists (False):
  ; //         - Gets the Spawner’s location (Get Actor Transform).
  ; //         - Spawns a new BP_NPC at that location.
  ; //         - Sets "Has NPC" to true.
  ; //         - Stores the spawned NPC reference in "Current NPC".
  ; //
  ; // Result: The Spawner only creates NPCs if none are active.
  ; // Ensures control to avoid duplicate spawns.
  (if (not (Variables|Default|GethasNPC))
    (bind _returnvalue (Game|SpawnActorfromClass "/Game/ThirdPerson/Blueprints/BP_NPC.BP_NPC_C" (Transformation|GetActorTransform) "Undefined" 0 (Variables|Default|GetExit%20Target%20Ref) 0))
    (Variables|Default|SethasNPC true)
    (Variables|Default|SetCurrentNPC _returnvalue)))

(event EventBeginPlay
  ;[1 1 1] 🇧🇷 Português
  ;
  ; // Sistema de Spawner de NPCs
  ; //
  ; // - Evento BeginPlay: Assim que o jogo começa, chama "Try Spawn NPC".
  ; // - TrySpawnNPC (Evento Personalizado):
  ; //     * Verifica a variável "Has NPC"
  ; //     * Se já existir um NPC (True), não faz nada.
  ; //     * Se não existir (False):
  ; //         - Pega a posição do Spawner (Get Actor Transform).
  ; //         - Cria (Spawn) um novo BP_NPC nessa posição.
  ; //         - Marca "Has NPC" como verdadeiro.
  ; //         - Salva a referência do NPC em "Current NPC".
  ; //
  ; // Resultado: O Spawner só cria NPCs se não houver nenhum ativo.
  ; // Garante controle para evitar spawns duplicados.
  ;
  ; 🇺🇸 English
  ;
  ; // NPC Spawner System
  ; //
  ; // - BeginPlay Event: When the game starts, calls "Try Spawn NPC".
  ; // - TrySpawnNPC (Custom Event):
  ; //     * Checks "Has NPC" variable.
  ; //     * If an NPC already exists (True), does nothing.
  ; //     * If none exists (False):
  ; //         - Gets the Spawner’s location (Get Actor Transform).
  ; //         - Spawns a new BP_NPC at that location.
  ; //         - Sets "Has NPC" to true.
  ; //         - Stores the spawned NPC reference in "Current NPC".
  ; //
  ; // Result: The Spawner only creates NPCs if none are active.
  ; // Ensures control to avoid duplicate spawns.
  (CallFunction|TrySpawnNPC))

(fn ConstructionScript)

(fn ResetHasNPC
  ;[1 1 1] 🇧🇷 Português
  ;
  ; // Sistema de Spawn de NPCs:
  ; // - "Reset Has NPC": Evento que reseta o estado de NPC
  ; // - Define a variável "Has NPC" como falso (false)
  ; // - Chama a função "Try Spawn NPC" no próprio Spawner
  ; //
  ; // Resultado: Sempre que for necessário resetar, o Spawner
  ; // verifica e tenta gerar (spawnar) um novo NPC no mundo.
  ;
  ; 🇺🇸 English
  ;
  ; // NPC Spawn System:
  ; // - "Reset Has NPC": Event that resets NPC state
  ; // - Sets the variable "Has NPC" to false
  ; // - Calls the function "Try Spawn NPC" on the Spawner itself
  ; //
  ; // Result: Whenever a reset is triggered, the Spawner
  ; // checks and tries to spawn a new NPC in the world.
  (Variables|Default|SethasNPC false)
  (CallFunction|TrySpawnNPC))